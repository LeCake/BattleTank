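; Tank pawn Blueprint that turns player input into tank movement, camera aiming and firing.
; On BeginPlay it hands its Barrel and Turret components to setter functions.
; Throttle axes drive each track directly, while MoveForward sends intent to the TankMovementComponent.
; Aim axes rotate the azimuth gimbal in yaw and the spring arm in pitch, and the Fire action calls Fire.
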(event `self.ReceiveBeginPlay`
  (`self.SetBarrelReference` (`self.Barrel`))
  (`self.SetTurretReference` (`self.Turret`)))

(event `InputAxis|AimAzimuth`
  (params (AxisValue :type "Float (single-precision)"))
  ;[1 1 1] Aiming input binding
  (`SceneComponent.K2_AddLocalRotation` (`self.Azimuth Gimbal`) (`KismetMathLibrary.MakeRotator` 0.0 0.0 AxisValue) false false))

(event `InputAxis|LeftTrackThrottle`
  (params (AxisValue :type "Float (single-precision)"))
  ;[1 1 1] Movement Input Binding
  (`TankTrack.SetThrottle` (`self.LeftTrack`) AxisValue))

(event `InputAxis|RightTrackThrottle`
  (params (AxisValue :type "Float (single-precision)"))
  ;[1 1 1] Movement Input Binding
  (`TankTrack.SetThrottle` (`self.RightTrack`) AxisValue))

(event `InputAxis|AimEleveation`
  (params (AxisValue :type "Float (single-precision)"))
  ;[1 1 1] Aiming input binding
  (`SceneComponent.K2_AddLocalRotation` (`self.Spring Arm`) (`KismetMathLibrary.MakeRotator` 0.0 AxisValue) false false))

(event `InputAxis|MoveForward`
  (params (AxisValue :type "Float (single-precision)"))
  ;[1 1 1] Movement Input Binding
  (`TankMovementComponent.IntentMoveFoward` (`self.TankMovementComponent`) AxisValue))

(event `InputAction|Fire`
  (params (Key :type "Key Structure"))
  ;[1 1 1] Aiming input binding
  (:`Pressed`
    (`self.Fire`)))

(fn `UserConstructionScript`)